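; Game state for a team deathmatch that tracks how many players remain alive on Team A and Team B.
; DecreaseTeamNumber lowers the chosen team's count and, when it reaches zero, shows a WB_TeamWinner widget naming the other team as winner.
; Otherwise UpdateWidget writes both counts to the local player character's HUD text, which also runs shortly after BeginPlay.
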(event `self.ReceiveBeginPlay`
  (`KismetSystemLibrary.Delay` 0.5)
  (`self.Update Widget`))

(event `Decrease Team Number`
  (params (`Team A` :type Boolean))
  (if `Team A`
    (bind _result (`/Engine/EditorBlueprintResources/StandardMacros.DecrementInt` (`self.numberOfTeamA_Alive`))
      (:`  `
        (if (<= _result 0)
          (bind _returnvalue (`|CreateWidget` "/Game/WB_TeamWinner.WB_TeamWinner_C"))
          (`TextBlock.SetText` (`/Game/WB_TeamWinner.WINNERTEXT` _returnvalue) "TEAM B WON")
          (`UserWidget.AddToViewport` _returnvalue 0)
          (else
            (`self.Update Widget` :!label _label)))))
    (else
      (bind _result_2 (`/Engine/EditorBlueprintResources/StandardMacros.DecrementInt` (`self.numberOfTeamB_Alive`))
        (:`  `
          (if (<= _result_2 0)
            (bind _returnvalue_2 (`|CreateWidget` "/Game/WB_TeamWinner.WB_TeamWinner_C"))
            (`TextBlock.SetText` (`/Game/WB_TeamWinner.WINNERTEXT` _returnvalue_2) "TEAM A WON")
            (`UserWidget.AddToViewport` _returnvalue_2 0)
            (else
              (goto _label))))))))

(event `Update Widget`
  (bind _asbp_third_person_character (cast `/Game/ThirdPerson/Blueprints/BP_ThirdPersonCharacter` (`GameplayStatics.GetPlayerCharacter` 0)))
  (bind _hud (`/Game/ThirdPerson/Blueprints/BP_ThirdPersonCharacter.HUD` _asbp_third_person_character))
  (`TextBlock.SetText` (`/Game/WB_HUD.TeamAText` _hud) (`|FormatText` "TEAM A: {Value}" (`self.numberOfTeamA_Alive`)))
  (`TextBlock.SetText` (`/Game/WB_HUD.TeamBText` _hud) (`|FormatText` "TEAM B: {Value}" (`self.numberOfTeamB_Alive`))))

(fn `UserConstructionScript`)